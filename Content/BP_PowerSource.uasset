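; BP_PowerSource is a spinning pickup that advances the mission text and sets a checkpoint when the player character touches it.
; Tick rotates the static mesh by a fixed step each frame, without delta-time scaling.
; Box overlap with BP_Character sets MissionTextNumber and MostRecentCheckPoint on SRGameModeMain, using the actor's own location as the checkpoint.
; The actor destroys itself after a short delay.
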(event OnComponentBeginOverlap(Box)
  (params (OverlappedComponent :type Primitive%20Component%20Object%20Reference) (OtherActor :type Actor%20Object%20Reference) (OtherComp :type Primitive%20Component%20Object%20Reference) (OtherBodyIndex :type Integer) (bFromSweep :type Boolean) (SweepResult :type Hit%20Result%20Structure%20%28by%20ref%29))
  (Utilities|Casting|CastToBP_Character OtherActor)
  (bind _assrgame_mode_main (Utilities|Casting|CastToSRGameModeMain (Game|GetGameMode)))
  (Variables|/Game/Core/SRGameModeMain.SRGameModeMain_C|SetMissionTextNumber _assrgame_mode_main 4)
  (Variables|/Game/Core/SRGameModeMain.SRGameModeMain_C|SetMostRecentCheckPoint _assrgame_mode_main (Transformation|GetActorLocation))
  (Utilities|FlowControl|Delay 0.1)
  (Actor|DestroyActor))

(event EventBeginPlay)

(event Collision|EventActorBeginOverlap
  (params (OtherActor :type Actor%20Object%20Reference)))

(event EventTick
  (params (DeltaSeconds :type Float%20%28single-precision%29))
  (Transformation|AddLocalRotation (Variables|Default|GetStaticMesh) "0.000000,-1.000000,0.000000" false false))

(fn ConstructionScript)