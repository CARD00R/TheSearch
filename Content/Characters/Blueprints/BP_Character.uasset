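; BP_Character is a shooter character Blueprint that handles a small amount of UI and debug feedback.
; On BeginPlay it adds the WBP_Crosshair widget to the viewport.
; SRHealth changes draw the health value as debug text at the character's location, and F toggles the FPS stat display.
; Disconnected leftover nodes cover starter gun spawning to GunSocket, slow motion and magazine ammo printing, and never run.
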(event OnHealthChanged(SRHealth)
  (params (HealthComp :type SR%20Health%20Component%20Object%20Reference) (Health :type Float%20%28single-precision%29) (HealthDelta :type Float%20%28single-precision%29) (DamageType :type Damage%20Type%20Object%20Reference) (InstigatedBy :type Controller%20Object%20Reference) (DamageCauser :type Actor%20Object%20Reference))
  (Rendering|Debug|DrawDebugString (Transformation|GetActorLocation) (Utilities|String|ToString(Float) Health) 0 "(R=1.000000,G=0.000000,B=0.035135,A=1.000000)" 2.0))

(event EventBeginPlay
  (Utilities|FlowControl|Sequence
    (:then_0
      (bind _returnvalue (UserInterface|CreateWidget "/Game/Characters/UI/WBP_Crosshair.WBP_Crosshair_C"))
      (UserInterface|Viewport|AddtoViewport _returnvalue 0))))

(event Collision|EventActorBeginOverlap
  (params (OtherActor :type Actor%20Object%20Reference)))

(event EventTick
  (params (DeltaSeconds :type Float%20%28single-precision%29)))

(event Input|KeyboardEvents|F
  (params (Key :type Key%20Structure :default "None"))
  (:Pressed
    (Development|ExecuteConsoleCommand "stat fps" 0)))

(fn ConstructionScript)