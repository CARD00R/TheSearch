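; BP_AdvancedAI is a human AI character with weapon and health hooks, driven by the BT_AdvancedAI behavior tree.
; BeginPlay starts the tree, caches the first BP_Character as Player and holsters the gun after a delay.
; Damage writes the causer's location to the blackboard as last known location, and a delayed Tick mirrors PrimaryWeapon ammo counts.
; Pawn sensing handlers are empty; combat and search modes remain a to-do note.
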(event OnHealthChanged(OwningHealthComp)
  (params (HealthComp :type SR%20Health%20Component%20Object%20Reference) (Health :type Float%20%28single-precision%29) (HealthDelta :type Float%20%28single-precision%29) (DamageType :type Damage%20Type%20Object%20Reference) (InstigatedBy :type Controller%20Object%20Reference) (DamageCauser :type Actor%20Object%20Reference))
  (AI|Components|Blackboard|SetValueasVector (AI|GetBlackboard (AI|GetAIController self)) (Variables|Default|GetBBKLastKnownLocation) (Transformation|GetActorLocation DamageCauser))
  (Development|PrintString "HIT"))

(event OnHearNoise(PawnSensing)
  (params (Instigator :type Pawn%20Object%20Reference) (Location :type Vector%20%28by%20ref%29 :default "0, 0, 0") (Volume :type Float%20%28single-precision%29)))

(event OnSeePawn(PawnSensing)
  (params (Pawn :type Pawn%20Object%20Reference)))

(event EventBeginPlay
  ;[0 0.4375 1] To Do:
  ; Combat Mode:
  ; -> Constantly looking for target, shooting behind cover that is a certain distance from player. If player is at a greater distance then RUN at player.
  ;
  ; NonCombat mode:
  ; -> Simply look around for player in adjustable radius
  (AI|RunBehaviorTree (AI|GetAIController self) "/Game/Characters/Blueprints/HumanAi/AIComponents/BT_AdvancedAI.BT_AdvancedAI")
  (bind _outactors (Actor|GetAllActorsOfClass "/Game/Characters/Blueprints/BP_Character.BP_Character_C"))
  (Variables|Default|SetPlayer (Utilities|Array|Get(acopy) _outactors))
  (Utilities|FlowControl|Delay 2.0)
  (Variables|Default|SetbGunHolstered true)
  (Utilities|FlowControl|Delay 1.0))

(event Collision|EventActorBeginOverlap
  (params (OtherActor :type Actor%20Object%20Reference)))

(event EventTick
  (params (DeltaSeconds :type Float%20%28single-precision%29))
  (bind _primaryweapon (Variables|Default|GetPrimaryWeapon))
  (Utilities|FlowControl|Delay 0.2)
  (Utilities|IsValid _primaryweapon
    (:Is%20Valid
      (Variables|Default|SetBulletsInMag (Variables|/Script/SpaceRaiders.SRGun|GetCurrentBulletsInMag _primaryweapon))
      (Variables|Default|SetBulletsInReserve (Variables|/Script/SpaceRaiders.SRGun|GetBulletsInReserve _primaryweapon)))))

(fn ConstructionScript)