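; BP_EntranceShield_OdinsVessel is a trigger box at the entrance to Odin's Vessel that reacts to overlaps by the SRSpaceShip.
; Behind a DoOnce, it toggles the ship's indoor speed multiplier and updates the game mode's mission text and hardcoded checkpoint location.
; Every ship overlap also checks Entered and, when it equals 2, destroys all valid Enemies actors; Entered is never changed in this graph.
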(event OnComponentBeginOverlap(Box)
  (params (OverlappedComponent :type Primitive%20Component%20Object%20Reference) (OtherActor :type Actor%20Object%20Reference) (OtherComp :type Primitive%20Component%20Object%20Reference) (OtherBodyIndex :type Integer) (bFromSweep :type Boolean) (SweepResult :type Hit%20Result%20Structure%20%28by%20ref%29))
  (bind _assrspace_ship (Utilities|Casting|CastToSRSpaceShip OtherActor))
  (Utilities|FlowControl|Sequence
    (:then_0
      (Utilities|FlowControl|DoOnce false
        (:Completed
          (if (> (Variables|/Script/SpaceRaiders.SRSpaceShip|GetIndoorSpeedChange _assrspace_ship) 0.6)
            (Variables|/Script/SpaceRaiders.SRSpaceShip|SetIndoorSpeedChange _assrspace_ship 0.5)
            (else
              (Variables|/Script/SpaceRaiders.SRSpaceShip|SetIndoorSpeedChange _assrspace_ship 0.8)))
          (bind _assrgame_mode_main (Utilities|Casting|CastToSRGameModeMain (Game|GetGameMode)))
          (Variables|/Game/Core/SRGameModeMain.SRGameModeMain_C|SetMissionTextNumber _assrgame_mode_main 3)
          (bind _assrgame_mode_main_2 (Utilities|Casting|CastToSRGameModeMain (Game|GetGameMode)))
          (Variables|/Game/Core/SRGameModeMain.SRGameModeMain_C|SetMostRecentCheckPoint _assrgame_mode_main_2 "14151.873047,3439.712402,-898.964722"))))
    (:then_1
      (if (== (Variables|Default|Getentered) 2)
        (for _array_element (Variables|Default|GetEnemies)
          (Utilities|IsValid _array_element
            (:Is%20Valid
              (Actor|DestroyActor _array_element))))))))

(event EventBeginPlay)

(event Collision|EventActorBeginOverlap
  (params (OtherActor :type Actor%20Object%20Reference)))

(event EventTick
  (params (DeltaSeconds :type Float%20%28single-precision%29)))

(fn ConstructionScript)