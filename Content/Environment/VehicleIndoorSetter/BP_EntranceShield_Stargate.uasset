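; BP_EntranceShield_Stargate is an entrance trigger that advances the mission when the player's spaceship reaches the stargate.
; The first ship overlap sets a hard-coded checkpoint and mission text on SRGameModeMain, adjusts the ship's IndoorSpeedChange and plays a beep.
; A counter increments on every box overlap, whatever the actor.
; On the second overlap, it destroys the Enemies list if mission text 2 is active.
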(event OnComponentBeginOverlap(Box)
  (params (OverlappedComponent :type Primitive%20Component%20Object%20Reference) (OtherActor :type Actor%20Object%20Reference) (OtherComp :type Primitive%20Component%20Object%20Reference) (OtherBodyIndex :type Integer) (bFromSweep :type Boolean) (SweepResult :type Hit%20Result%20Structure%20%28by%20ref%29))
  (Math|Integer|IncrementInt (Variables|Default|Getentered)
    (:%20%20
      (Utilities|FlowControl|Sequence
        (:then_0
          (bind _assrspace_ship (Utilities|Casting|CastToSRSpaceShip OtherActor))
          (Utilities|FlowControl|DoOnce false
            (:Completed
              (bind _assrgame_mode_main (Utilities|Casting|CastToSRGameModeMain (Game|GetGameMode)))
              (Variables|/Game/Core/SRGameModeMain.SRGameModeMain_C|SetMostRecentCheckPoint _assrgame_mode_main "-1189246.375000,-330806.750000,36303.328125")
              (if (> (Variables|/Script/SpaceRaiders.SRSpaceShip|GetIndoorSpeedChange _assrspace_ship) 0.6)
                (Variables|/Script/SpaceRaiders.SRSpaceShip|SetIndoorSpeedChange _assrspace_ship 0.5)
                (else
                  (Variables|/Script/SpaceRaiders.SRSpaceShip|SetIndoorSpeedChange _assrspace_ship 0.8)))
              (bind _assrgame_mode_main_2 (Utilities|Casting|CastToSRGameModeMain (Game|GetGameMode)))
              (Variables|/Game/Core/SRGameModeMain.SRGameModeMain_C|SetMissionTextNumber _assrgame_mode_main_2 1)
              (Audio|PlaySound2D "/Game/UI/Beep_Cue.Beep_Cue" 1.0 1.0 0.0 0 0))))
        (:then_1
          (if (== (Variables|Default|Getentered) 2)
            (bind _assrgame_mode_main_3 (Utilities|Casting|CastToSRGameModeMain (Game|GetGameMode)))
            (if (== (Variables|/Game/Core/SRGameModeMain.SRGameModeMain_C|GetMissionTextNumber _assrgame_mode_main_3) 2)
              (for _array_element (Variables|Default|GetEnemies)
                (Utilities|IsValid _array_element
                  (:Is%20Valid
                    (Actor|DestroyActor _array_element)))))))))))

(event EventBeginPlay)

(event Collision|EventActorBeginOverlap
  (params (OtherActor :type Actor%20Object%20Reference)))

(event EventTick
  (params (DeltaSeconds :type Float%20%28single-precision%29)))

(fn ConstructionScript)