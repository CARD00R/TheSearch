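; Vulkan spaceship vehicle Blueprint that drives thruster and boost glow from the ship's speed.
; Each Tick creates new dynamic material instances on ShipMesh and sets Emissive Power from horizontal velocity and IsBoosting.
; SpaceBar latches Clamp, switching the glow scaling and enabling boost camera shake; otherwise scaled speed prints as debug.
; Left Alt takes a 4K screenshot, while the character-interaction overlap logic is disconnected.
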(event OnComponentBeginOverlap(InteractCollision)
  (params (OverlappedComponent :type Primitive%20Component%20Object%20Reference) (OtherActor :type Actor%20Object%20Reference) (OtherComp :type Primitive%20Component%20Object%20Reference) (OtherBodyIndex :type Integer) (bFromSweep :type Boolean) (SweepResult :type Hit%20Result%20Structure%20%28by%20ref%29)))

(event OnComponentEndOverlap(InteractCollision)
  (params (OverlappedComponent :type Primitive%20Component%20Object%20Reference) (OtherActor :type Actor%20Object%20Reference) (OtherComp :type Primitive%20Component%20Object%20Reference) (OtherBodyIndex :type Integer)))

(event EventBeginPlay
  ;[0 0.4609 1] Boost / Thrust Materials
)

(event Collision|EventActorBeginOverlap
  (params (OtherActor :type Actor%20Object%20Reference))
  ;[0 0.4609 1] Boost / Thrust Materials
)

(event EventTick
  (params (DeltaSeconds :type Float%20%28single-precision%29))
  (bind _returnvalue (Transformation|GetVelocity))
  (bind _returnvalue_2 (Transformation|GetVelocity))
  (bind (_x _y) (Math|Vector|BreakVector _returnvalue))
  (bind (_x_2 _y_2) (Math|Vector|BreakVector _returnvalue_2))
  (bind _returnvalue_3 (Math|Vector|MakeVector _x _y 0.0))
  (bind _returnvalue_4 (Math|Vector|MakeVector _x_2 _y_2 0.0))
  (bind _returnvalue_5 (Math|Vector|VectorLength _returnvalue_3))
  (bind _returnvalue_6 (Math|Vector|VectorLength _returnvalue_4))
  (bind _returnvalue_7 (/ _returnvalue_5 5.0))
  (bind _returnvalue_8 (/ _returnvalue_6 5e+02))
  ;[0 0.4609 1] Boost / Thrust Materials
  (if (Variables|Default|GetClamp)
    (Utilities|FlowControl|Sequence
      (:then_0
        (bind _returnvalue_9 (Rendering|Material|CreateDynamicMaterialInstance (Variables|Default|GetShipMesh) 1 "/Game/Vehicles/SpaceShips/Vulkan/Materials/MatInst_V_SS_Vulkan_Thrust.MatInst_V_SS_Vulkan_Thrust" "None" :!class /Script/Engine.PrimitiveComponent))
        (Rendering|Material|SetScalarParameterValue _returnvalue_9 "Emissive Power" (Math|Float|Clamp(Float) _returnvalue_7 3.0 1.3e+02) :!class /Script/Engine.MaterialInstanceDynamic))
      (:then_1
        (if (Variables|Default|GetbIsBoosting)
          (bind _returnvalue_10 (Rendering|Material|CreateDynamicMaterialInstance (Variables|Default|GetShipMesh) 2 "/Game/Vehicles/SpaceShips/Vulkan/Materials/MatInst_V_SS_Vulkan_Boost.MatInst_V_SS_Vulkan_Boost" "None" :!class /Script/Engine.PrimitiveComponent))
          (Rendering|Material|SetScalarParameterValue _returnvalue_10 "Emissive Power" (/ _returnvalue_7 6e+01) :!class /Script/Engine.MaterialInstanceDynamic)
          (else
            (bind _returnvalue_11 (Rendering|Material|CreateDynamicMaterialInstance (Variables|Default|GetShipMesh) 2 "/Game/Vehicles/SpaceShips/Vulkan/Materials/MatInst_V_SS_Vulkan_Boost.MatInst_V_SS_Vulkan_Boost" "None" :!class /Script/Engine.PrimitiveComponent))
            (Rendering|Material|SetScalarParameterValue _returnvalue_11 "Emissive Power" 5e+01 :!class /Script/Engine.MaterialInstanceDynamic))))
      (:then_2
        (if (Variables|Default|GetbIsBoosting)
          (Class|PlayerController|ClientPlayCameraShake (Game|GetPlayerController 0) "/Game/Vehicles/SpaceShips/Vulkan/Effects/CS_Speed2.CS_Speed2_C" 1.0 "CameraLocal" "0, 0, 0"))))
    (else
      (Utilities|FlowControl|Sequence
        (:then_0
          (bind _returnvalue_12 (Rendering|Material|CreateDynamicMaterialInstance (Variables|Default|GetShipMesh) 1 "/Game/Vehicles/SpaceShips/Vulkan/Materials/MatInst_V_SS_Vulkan_Thrust.MatInst_V_SS_Vulkan_Thrust" "None" :!class /Script/Engine.PrimitiveComponent))
          (Rendering|Material|SetScalarParameterValue _returnvalue_12 "Emissive Power" (Math|Float|Clamp(Float) _returnvalue_8 0.0 9e+01) :!class /Script/Engine.MaterialInstanceDynamic)
          (Development|PrintString (Utilities|String|ToString(Float) _returnvalue_8) true false "(R=0.000000,G=0.660000,B=1.000000,A=1.000000)" 0.0))
        (:then_1
          (if (Variables|Default|GetbIsBoosting)
            (bind _returnvalue_13 (Rendering|Material|CreateDynamicMaterialInstance (Variables|Default|GetShipMesh) 2 "/Game/Vehicles/SpaceShips/Vulkan/Materials/MatInst_V_SS_Vulkan_Boost.MatInst_V_SS_Vulkan_Boost" "None" :!class /Script/Engine.PrimitiveComponent))
            (Rendering|Material|SetScalarParameterValue _returnvalue_13 "Emissive Power" (/ _returnvalue_8 5.0) :!class /Script/Engine.MaterialInstanceDynamic)
            (else
              (bind _returnvalue_14 (Rendering|Material|CreateDynamicMaterialInstance (Variables|Default|GetShipMesh) 2 "/Game/Vehicles/SpaceShips/Vulkan/Materials/MatInst_V_SS_Vulkan_Boost.MatInst_V_SS_Vulkan_Boost" "None" :!class /Script/Engine.PrimitiveComponent))
              (Rendering|Material|SetScalarParameterValue _returnvalue_14 "Emissive Power" (Math|Float|Clamp(Float) _returnvalue_8) :!class /Script/Engine.MaterialInstanceDynamic))))))))

(event Input|KeyboardEvents|SpaceBar
  (params (Key :type Key%20Structure :default "None"))
  (:Pressed
    (Variables|Default|SetClamp true)))

(event Input|KeyboardEvents|LeftAlt
  (params (Key :type Key%20Structure :default "None"))
  (:Pressed
    (Development|ExecuteConsoleCommand "HighResShot 3840x2160" 0)))

(fn ConstructionScript)